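; Elevator Blueprint that moves its platform between start and end locations when a Character enters its trigger box.
; A repeatedly restarted timeline lerps height by MovePerSecond in the current direction, plus a fixed upward offset, stopping within tolerance of the target.
; DoOnce guards the trigger.
; A Character leaving the box resets it, toggles GoingDown and swaps the target, even mid-ride.
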(event `self.ReceiveBeginPlay`
  (set `self.ElevatorTargetLocation` (`SceneComponent.K2_GetComponentLocation` (`self.EndLocation`))))

(event `self.Box.OnComponentBeginOverlap`
  (params (OverlappedComponent :type "PrimitiveComponent Object Reference") (OtherActor :type "Actor Object Reference") (OtherComp :type "PrimitiveComponent Object Reference") (OtherBodyIndex :type Integer) (bFromSweep :type Boolean) (SweepResult :type "HitResult Structure (by ref)"))
  (bind _elevatorlocation (`self.ElevatorLocation`))
  (bind _returnvalue (not (== (`SceneComponent.K2_GetComponentLocation` (`self.Elevator`)) (`self.ElevatorTargetLocation`) :`ErrorTolerance` 10.0)))
  (cast `Character` OtherActor)
  (`/Engine/EditorBlueprintResources/StandardMacros.DoOnce` false :!label _label
    (:`Completed`
      (set `self.ElevatorLocation` (`SceneComponent.K2_GetComponentLocation` (`self.Elevator`)) :!label _label_2)
      (bind (_direction _persecond) (`Timeline|MoveElevator` :!via `PlayFromStart` :!label _label_3)
        (:`Update`
          (if _returnvalue
            (`SceneComponent.K2_SetWorldLocation` (`self.Elevator`) (`KismetMathLibrary.VLerp` _elevatorlocation (`KismetMathLibrary.MakeVector` (.x _elevatorlocation) (.y _elevatorlocation) (+ (.z _elevatorlocation) (* (`self.MovePerSecond`) (`KismetMathLibrary.SelectFloat` -1.0 1.0 (`self.GoingDown`))) 100.0)) _persecond) false false)
            (else
              (`self.HasReachedLocation` :!label _label_4))))
        (:`Finished`
          (if _returnvalue
            (goto _label_2)
            (else
              (goto _label_4))))))))

(event `HasReachedLocation`
  (goto _label_3 :!via `Stop`))

(event `self.Box.OnComponentEndOverlap`
  (params (OverlappedComponent :type "PrimitiveComponent Object Reference") (OtherActor :type "Actor Object Reference") (OtherComp :type "PrimitiveComponent Object Reference") (OtherBodyIndex :type Integer))
  (cast `Character` OtherActor)
  (`|ExecutionSequence`
    (:`then_0`
      (goto _label :!via `Reset`))
    (:`then_1`
      (set `self.GoingDown` (select `bool` (`self.GoingDown`) :`false` true))
      (`/Engine/EditorBlueprintResources/StandardMacros.FlipFlop`
        (:`A`
          (set `self.ElevatorTargetLocation` (`SceneComponent.K2_GetComponentLocation` (`self.StartLocation`))))
        (:`B`
          (set `self.ElevatorTargetLocation` (`SceneComponent.K2_GetComponentLocation` (`self.EndLocation`))))))))

(fn `UserConstructionScript`)